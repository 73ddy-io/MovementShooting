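; BP_BaseCharacter is a base character Blueprint that provides player movement, mouse look and jumping.
; Axis inputs move the character along its actor forward and right vectors and feed look input into controller pitch and yaw.
; The Jump action triggers the character's jump on press, and the construction script is empty.
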(event Input|ActionEvents|InputActionJump
  (params (Key :type Key%20Structure :default "None"))
  ;[0.62 0.01511 0.000794 1 25] Moving and Jumping
  (:Pressed
    (Character|Jump)))

(event Input|AxisEvents|InputAxisMoveBackAndForth
  (params (AxisValue :type Float%20%28single-precision%29))
  ;[0.62 0.01511 0.000794 1 25] Moving and Jumping
  (Pawn|Input|AddMovementInput (Transformation|GetActorForwardVector) AxisValue false))

(event Input|AxisEvents|InputAxisMoveSideToSide
  (params (AxisValue :type Float%20%28single-precision%29))
  ;[0.62 0.01511 0.000794 1 25] Moving and Jumping
  (Pawn|Input|AddMovementInput (Transformation|GetActorRightVector) AxisValue false))

(event Input|AxisEvents|InputAxisLookUp
  (params (AxisValue :type Float%20%28single-precision%29))
  ;[0.7992 0.1766 0 1 25] RotatingMouse
  (Pawn|Input|AddControllerPitchInput AxisValue))

(event Input|AxisEvents|InputAxisTurnAround
  (params (AxisValue :type Float%20%28single-precision%29))
  ;[0.7992 0.1766 0 1 25] RotatingMouse
  (Pawn|Input|AddControllerYawInput AxisValue))

(fn ConstructionScript)